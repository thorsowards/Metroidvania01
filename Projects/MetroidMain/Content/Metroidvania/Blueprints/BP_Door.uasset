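; BP_Door is a two-sided Metroidvania door that moves the player between adjacent rooms.
; After a one-tick delay on BeginPlay, it caches the first camera overlapping each spawn location as that side's camera.
; Overlapping either trigger flags the character as moving through a door, assigns the opposite side's spawn position and camera, then calls RoomTransition on the game mode.
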(event `self.ReceiveBeginPlay`
  ;[0 0 0] Get Cameras
  (`KismetSystemLibrary.Delay` 0.0)
  (bind _asbp_metroidvania_camera (cast `/Game/Metroidvania/Blueprints/BP_MetroidvaniaCamera` (`|GetArrayItem` (`PrimitiveComponent.GetOverlappingActors` (`self.RightSpawnLocation`) "/Game/Metroidvania/Blueprints/BP_MetroidvaniaCamera.BP_MetroidvaniaCamera_C"))))
  (set `self.RightCamera` _asbp_metroidvania_camera)
  (bind _asbp_metroidvania_camera_2 (cast `/Game/Metroidvania/Blueprints/BP_MetroidvaniaCamera` (`|GetArrayItem` (`PrimitiveComponent.GetOverlappingActors` (`self.LeftSpawnLocation`) "/Game/Metroidvania/Blueprints/BP_MetroidvaniaCamera.BP_MetroidvaniaCamera_C"))))
  (set `self.LeftCamera` _asbp_metroidvania_camera_2))

(event `self.DoorTriggerRight.OnComponentBeginOverlap`
  (params (OverlappedComponent :type "PrimitiveComponent Object Reference") (OtherActor :type "Actor Object Reference") (OtherComp :type "PrimitiveComponent Object Reference") (OtherBodyIndex :type Integer) (bFromSweep :type Boolean) (SweepResult :type "HitResult Structure (by ref)"))
  ;[0 0 0] Door Triggers
  (bind _asbp_metroidvania_character (cast `/Game/Metroidvania/Blueprints/BP_MetroidvaniaCharacter` OtherActor))
  (set `/Game/Metroidvania/Blueprints/BP_MetroidvaniaCharacter.IsMovingThroughDoor` true _asbp_metroidvania_character)
  (set `/Game/Metroidvania/Blueprints/BP_MetroidvaniaCharacter.NewSpawnPosition` (`SceneComponent.K2_GetComponentLocation` (`self.LeftSpawnLocation`)) _asbp_metroidvania_character)
  (set `/Game/Metroidvania/Blueprints/BP_MetroidvaniaCharacter.CurrentCam` (`self.LeftCamera`) _asbp_metroidvania_character)
  (bind _asbp_metroidvania_game_mode (cast `/Game/Metroidvania/Blueprints/BP_MetroidvaniaGameMode` (`GameplayStatics.GetGameMode`) :!label _label))
  (`/Game/Metroidvania/Blueprints/BP_MetroidvaniaGameMode.RoomTransition` _asbp_metroidvania_game_mode))

(event `self.DoorTriggerLeft.OnComponentBeginOverlap`
  (params (OverlappedComponent :type "PrimitiveComponent Object Reference") (OtherActor :type "Actor Object Reference") (OtherComp :type "PrimitiveComponent Object Reference") (OtherBodyIndex :type Integer) (bFromSweep :type Boolean) (SweepResult :type "HitResult Structure (by ref)"))
  ;[0 0 0] Door Triggers
  (bind _asbp_metroidvania_character (cast `/Game/Metroidvania/Blueprints/BP_MetroidvaniaCharacter` OtherActor))
  (set `/Game/Metroidvania/Blueprints/BP_MetroidvaniaCharacter.IsMovingThroughDoor` true _asbp_metroidvania_character)
  (set `/Game/Metroidvania/Blueprints/BP_MetroidvaniaCharacter.NewSpawnPosition` (`SceneComponent.K2_GetComponentLocation` (`self.RightSpawnLocation`)) _asbp_metroidvania_character)
  (set `/Game/Metroidvania/Blueprints/BP_MetroidvaniaCharacter.CurrentCam` (`self.RightCamera`) _asbp_metroidvania_character)
  (goto _label))

(fn `UserConstructionScript`)