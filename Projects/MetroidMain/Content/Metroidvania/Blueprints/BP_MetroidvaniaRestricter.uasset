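; BP_MetroidvaniaRestricter is a placeable camera confinement zone for the Metroidvania side-view camera.
; The construction script shapes the player trigger and sizes the confines box in multiples of a 16:9 screen of 16-unit tiles.
; On BeginPlay it derives X/Z camera limits by insetting that box by half a screen.
; Trigger overlaps by BP_MetroidvaniaCharacter activate or deactivate the restricter on that character's current camera.
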(event `self.ReceiveBeginPlay`
  (`self.GetConfinesBoxBounds`))

(event `self.PlayerTriggerBox.OnComponentBeginOverlap`
  (params (OverlappedComponent :type "PrimitiveComponent Object Reference") (OtherActor :type "Actor Object Reference") (OtherComp :type "PrimitiveComponent Object Reference") (OtherBodyIndex :type Integer) (bFromSweep :type Boolean) (SweepResult :type "HitResult Structure (by ref)"))
  (bind _asbp_metroidvania_character (cast `/Game/Metroidvania/Blueprints/BP_MetroidvaniaCharacter` OtherActor))
  (`/Game/Metroidvania/Blueprints/BP_MetroidvaniaCamera.SetRestricterActive` (`/Game/Metroidvania/Blueprints/BP_MetroidvaniaCharacter.CurrentCam` _asbp_metroidvania_character) self))

(event `self.PlayerTriggerBox.OnComponentEndOverlap`
  (params (OverlappedComponent :type "PrimitiveComponent Object Reference") (OtherActor :type "Actor Object Reference") (OtherComp :type "PrimitiveComponent Object Reference") (OtherBodyIndex :type Integer))
  (bind _asbp_metroidvania_character (cast `/Game/Metroidvania/Blueprints/BP_MetroidvaniaCharacter` OtherActor))
  (`/Game/Metroidvania/Blueprints/BP_MetroidvaniaCamera.SetRestricterInactive` (`/Game/Metroidvania/Blueprints/BP_MetroidvaniaCharacter.CurrentCam` _asbp_metroidvania_character) self))

(fn `UserConstructionScript`
  (`SceneComponent.K2_SetRelativeTransform` (`self.PlayerTriggerBox`) (`self.PlayerTriggerTransform`) false false)
  (`BoxComponent.SetBoxExtent` (`self.PlayerTriggerBox`) (`self.PlayerTriggerExtent`) true)
  (`BoxComponent.SetBoxExtent` (`self.CameraConfinesBox`) (`KismetMathLibrary.MakeVector` (`KismetMathLibrary.Conv_IntToDouble` (* (* (`self.ConfinerWidth`) 8) 16)) 10.0 (`KismetMathLibrary.Conv_IntToDouble` (* (* (`self.ConfinerHeight`) 8) 9))) true))