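; Player character for a Metroidvania-style game, a side-view flipbook sprite that runs and jumps along the X axis.
; On start it finds the overlapping BP_MetroidvaniaCamera and makes it the view target.
; Movement flips control yaw to face the travel direction, and movement and jump input are ignored while IsMovingThroughDoor is set.
; Tick picks Idle or Run when grounded, while jumping switches to Falling after a short delay.
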(event `self.ReceiveBeginPlay`
  ;[0 0 0] Get Starting Cam
  (`KismetSystemLibrary.Delay` 0.0)
  (bind _asbp_metroidvania_camera (cast `/Game/Metroidvania/Blueprints/BP_MetroidvaniaCamera` (`|GetArrayItem` (`PrimitiveComponent.GetOverlappingActors` (`self.CapsuleComponent`) "/Game/Metroidvania/Blueprints/BP_MetroidvaniaCamera.BP_MetroidvaniaCamera_C"))))
  (bind _output_get (set `self.CurrentCam` _asbp_metroidvania_camera))
  (`PlayerController.SetViewTargetWithBlend` (`GameplayStatics.GetPlayerController` 0) _output_get 0.0 "VTBlend_Linear" 0.0 false))

(event `InputAxis|MoveRight`
  (params (AxisValue :type "Float (single-precision)"))
  (bind _returnvalue (`self.GetController`))
  ;[0 0 0] Movement
  (if (not (`self.IsMovingThroughDoor`))
    (`/Engine/EditorBlueprintResources/StandardMacros.CompareFloat` AxisValue
      (:`>`
        (set `self.IsMovingRight` true))
      (:`<`
        (set `self.IsMovingRight` false)))
    (`self.AddMovementInput` (1.0 0.0 0.0) AxisValue)
    (if (`self.IsMovingRight`)
      (`Controller.SetControlRotation` _returnvalue (`KismetMathLibrary.MakeRotator` 0.0))
      (else
        (`Controller.SetControlRotation` _returnvalue (`KismetMathLibrary.MakeRotator` 0.0 0.0 180.0))))))

(event `InputAction|Jump`
  (params (Key :type "Key Structure"))
  (bind _ismovingthroughdoor (`self.IsMovingThroughDoor`))
  ;[0 0 0] Jumping
  (:`Pressed`
    (if (not _ismovingthroughdoor)
      (`self.Jump`)
      (if (`self.CanJump`)
        (`self.SetAnimationState` "NewEnumerator0")
        (`KismetSystemLibrary.Delay` 0.2)
        (if (`NavMovementComponent.IsFalling` (`self.CharacterMovement`))
          (`self.SetAnimationState` "NewEnumerator3")))))
  (:`Released`
    (if (not _ismovingthroughdoor)
      (`self.StopJumping`))))

(event `self.ReceiveTick`
  (params (DeltaSeconds :type "Float (single-precision)"))
  ;[0 0 0] Set Animation
  (if (not (`NavMovementComponent.IsFalling` (`self.CharacterMovement`)))
    (`self.SetAnimationState` (select `bool` (> (`KismetMathLibrary.VSize` (`self.GetVelocity`)) 0.0) :`false` "NewEnumerator0" :`true` "NewEnumerator1" :!type "/Game/Metroidvania/Blueprints/AnimationStates Enum"))))

(fn `SetAnimationState`
  (params (AnimState :type "/Game/Metroidvania/Blueprints/AnimationStates Enum" :default "NewEnumerator0"))
  (set `self.CurrentAnimationState` AnimState)
  (`PaperFlipbookComponent.SetFlipbook` (`self.Sprite`) (select `/Game/Metroidvania/Blueprints/AnimationStates` (`self.CurrentAnimationState`) :`NewEnumerator0` (`self.Idle`) :`NewEnumerator1` (`self.Run`) :`NewEnumerator2` (`self.Jumping`) :`NewEnumerator3` (`self.Falling`)))
  (return))

(fn `UserConstructionScript`)