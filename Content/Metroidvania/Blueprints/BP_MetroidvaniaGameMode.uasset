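; Game mode for the Metroidvania game that runs the door-to-room transition for the player character.
; RoomTransition flags the character as moving through a door, then a timeline drives a shared material parameter collection Opacity value to fade sprites out.
; It teleports the player to the character's stored spawn position and blends the view to its current camera.
; After the blend, a second timeline fades sprites back in and clears the flag.
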(event `RoomTransition`
  ;[0 0 0] Lock and Hide
  (bind _asbp_metroidvania_character (cast `/Game/Metroidvania/Blueprints/BP_MetroidvaniaCharacter` (`GameplayStatics.GetPlayerPawn` 0)))
  (set `/Game/Metroidvania/Blueprints/BP_MetroidvaniaCharacter.IsMovingThroughDoor` true _asbp_metroidvania_character)
  ;[0 0 0] Fade Out Sprites
  (bind (_direction _opacity) (`Timeline|SpriteFadeOutTimeline` :!via `PlayFromStart`)
    (:`Update`
      (`KismetMaterialLibrary.SetScalarParameterValue` "/Game/Metroidvania/Materials/MetroidvaniaParamCollection.MetroidvaniaParamCollection" "Opacity" (`KismetMathLibrary.Lerp` 0.0 1.0 _opacity)))
    (:`OnComplete`
      ;[0 0 0] Teleport and Show Player
      (`self.K2_TeleportTo` :`self` _asbp_metroidvania_character :`DestLocation` (`/Game/Metroidvania/Blueprints/BP_MetroidvaniaCharacter.NewSpawnPosition` _asbp_metroidvania_character))
      (`PlayerController.SetViewTargetWithBlend` (`GameplayStatics.GetPlayerController` 0) (`/Game/Metroidvania/Blueprints/BP_MetroidvaniaCharacter.CurrentCam` _asbp_metroidvania_character) 0.75 "VTBlend_EaseInOut" 2.0 false)
      ;[0 0 0] Wait for Camera Tranisition
      (`KismetSystemLibrary.Delay` 0.75)
      ;[0 0 0] Fade Sprites In
      (bind (_direction_2 _opacity_2) (`Timeline|SpriteFadeInTimeline` :!via `PlayFromStart`)
        (:`Update`
          (`KismetMaterialLibrary.SetScalarParameterValue` "/Game/Metroidvania/Materials/MetroidvaniaParamCollection.MetroidvaniaParamCollection" "Opacity" (`KismetMathLibrary.Lerp` 1.0 0.0 _opacity_2)))
        (:`OnComplete`
          ;[0 0 0] Unlock Player
          (set `/Game/Metroidvania/Blueprints/BP_MetroidvaniaCharacter.IsMovingThroughDoor` false _asbp_metroidvania_character))))))

(fn `UserConstructionScript`)